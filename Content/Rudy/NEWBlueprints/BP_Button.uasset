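; BP_Button is an interactable button that opens a door when the disc is held.
; BeginPlay creates a P_Interact1 prompt and caches the first BP_Door and BP_Disc found in the level.
; The box overlap shows the prompt for the player and hides it on any end overlap, as that check compares the player to itself.
; NewFunction, not called within this Blueprint, checks IsHeld, opens the door and removes the prompt.
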(event `/Game/Destruction/BPI_OnInteract.NewFunction`
  (if (`/Game/Rudy/BP_Disc.IsHeld` (`self.BP_Disc`))
    (`/Game/Rudy/NEWBlueprints/BP_Door.OpenDoor` (`self.BP_Door`))
    (`Widget.RemoveFromParent` (`self.InteractPrompt`))))

(event `self.ReceiveBeginPlay`
  (bind _returnvalue (`|CreateWidget` "/Game/Rudy/P_Interact1.P_Interact1_C"))
  (set `self.InteractPrompt` _returnvalue)
  (`|ExecutionSequence`
    (:`then_0`
      (bind _outactors (`GameplayStatics.GetAllActorsOfClass` "/Game/Rudy/NEWBlueprints/BP_Door.BP_Door_C"))
      (for _array_element _outactors
        (set `self.BP_Door` _array_element)
        (break)))
    (:`then_1`
      (bind _outactors_2 (`GameplayStatics.GetAllActorsOfClass` "/Game/Rudy/BP_Disc.BP_Disc_C"))
      (for _array_element_2 _outactors_2
        (set `self.BP_Disc` _array_element_2)
        (break)))))

(event `self.Box.OnComponentBeginOverlap`
  (params (OverlappedComponent :type "PrimitiveComponent Object Reference") (OtherActor :type "Actor Object Reference") (OtherComp :type "PrimitiveComponent Object Reference") (OtherBodyIndex :type Integer) (bFromSweep :type Boolean) (SweepResult :type "HitResult Structure (by ref)"))
  (if (== OtherActor (`GameplayStatics.GetPlayerCharacter` 0))
    (`UserWidget.AddToViewport` (`self.InteractPrompt`) 0)))

(event `self.Box.OnComponentEndOverlap`
  (params (OverlappedComponent :type "PrimitiveComponent Object Reference") (OtherActor :type "Actor Object Reference") (OtherComp :type "PrimitiveComponent Object Reference") (OtherBodyIndex :type Integer))
  (if (== (`GameplayStatics.GetPlayerCharacter` 0) (`GameplayStatics.GetPlayerCharacter` 0))
    (`Widget.RemoveFromParent` (`self.InteractPrompt`))))

(fn `UserConstructionScript`)