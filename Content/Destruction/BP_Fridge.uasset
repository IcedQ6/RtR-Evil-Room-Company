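; BP_Fridge is a destructible fridge actor with an unfinished check for whether the BP_RudyKey actor is held.
; BeginPlay caches the first BP_RudyKey found in the level, and the NewFunction event reads its IsHeld flag, printing the result as debug text.
; Geometry collection strain and velocity calls and a text render update sit unwired, so the event triggers no destruction.
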(event `self.ReceiveBeginPlay`
  (bind _outactors (`GameplayStatics.GetAllActorsOfClass` "/Game/Destruction/BP_RudyKey.BP_RudyKey_C"))
  (for _array_element _outactors
    (set `self.Rudy Key` _array_element)
    (break)))

(event `/Game/Destruction/BPI_OnInteract.NewFunction`
  (if (`/Game/Destruction/BP_RudyKey.IsHeld` (`self.Rudy Key`))
    (`KismetSystemLibrary.PrintString` "Held")
    (else
      (`KismetSystemLibrary.PrintString` "Not held!"))))

(fn `UserConstructionScript`)